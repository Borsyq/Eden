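; Labyrinth minigame door that opens once the player has collected enough crystals.
; Overlap on the CrystalAmountChecker component casts to BP_ThirdPersonCharacter and compares its TotalCrystalsCollected with RequiredCrystalAmount.
; On success, the DoorActivation timeline drives the door mesh's relative Z and activates VFX on each update.
; Otherwise it adds a new Find_10crystals hint widget to the viewport on each overlap, with no removal here.
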(event OnComponentBeginOverlap(CrystalAmountChecker)
  (params (OverlappedComponent :type Primitive%20Component%20Object%20Reference) (OtherActor :type Actor%20Object%20Reference) (OtherComp :type Primitive%20Component%20Object%20Reference) (OtherBodyIndex :type Integer) (bFromSweep :type Boolean) (SweepResult :type Hit%20Result%20Structure%20%28by%20ref%29))
  (bind _asbp_third_person_character (Utilities|Casting|CastToBP_ThirdPersonCharacter OtherActor))
  (if (>= (Variables|/Game/ThirdPerson/Blueprints/BP_ThirdPersonCharacter.BP_ThirdPersonCharacter_C|GetTotalCrystalsCollected _asbp_third_person_character) (Variables|Default|GetRequiredCrystalAmount))
    (bind _door_activation (Timeline|Door%20Activation Play)
      (:Update
        (Transformation|SetRelativeLocation (Variables|Default|GetDoor%20Mesh) (Math|Vector|MakeVector -62.094456 295.442324 _door_activation) false false)
        (Components|Activation|Activate (Variables|Default|GetVFX) false)))
    (else
      (bind _returnvalue (UserInterface|CreateWidget "/Game/UI_Widget/UI_Files/Widget/Find_10crystals.Find_10crystals_C"))
      (UserInterface|Viewport|AddtoViewport _returnvalue 0))))

(fn ConstructionScript)
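; Labyrinth minigame door that moves vertically in response to pressure switch activation and deactivation events.
; Each event adjusts an active-switch count and plays or reverses a timeline that drives the door's relative Z, with X and Y hard-coded.
; The count is compared against zero, leaving PressureSwitchesNeeded unused, so at non-negative counts activation plays the timeline and deactivation reverses it.
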(event Custom|Switch%20Deactivated
  (Math|Integer|DecrementInt (Variables|Default|GetPressure%20Switches%20Active)
    (:%20%20
      (if (>= (Variables|Default|GetPressure%20Switches%20Active) 0)
        (bind _door_activation (Timeline|Timeline Reverse)
          (:Update
            (Transformation|SetRelativeLocation (Variables|Default|GetDoor) (Math|Vector|MakeVector 1.011e+04 -3.3e+03 _door_activation) false false)))
        (else
          (Timeline|Timeline Play))))))

(event Custom|Switch%20Activated
  (Math|Integer|IncrementInt (Variables|Default|GetPressure%20Switches%20Active)
    (:%20%20
      (if (>= (Variables|Default|GetPressure%20Switches%20Active) 0)
        (bind _door_activation (Timeline|Timeline Play)
          (:Update
            (Transformation|SetRelativeLocation (Variables|Default|GetDoor) (Math|Vector|MakeVector 1.011e+04 -3.3e+03 _door_activation) false false)))
        (else
          (Timeline|Timeline Reverse))))))

(fn ConstructionScript)
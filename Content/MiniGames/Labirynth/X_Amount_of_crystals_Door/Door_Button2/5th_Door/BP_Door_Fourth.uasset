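; BP_Door_Fourth is a labyrinth minigame door that moves in response to pressure switch events.
; SwitchActivated and SwitchDeactivated adjust an active-switch counter, then play or reverse the DoorActivation timeline, which drives the mesh's relative Z at fixed X and Y.
; Both events compare the counter against zero, with PressureSwitchesNeeded left unused, so activation plays and deactivation reverses while the count stays non-negative.
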(event Custom|Switch%20Deactivated
  (Math|Integer|DecrementInt (Variables|Default|GetPressure%20Switches%20Active)
    (:%20%20
      (if (>= (Variables|Default|GetPressure%20Switches%20Active) 0)
        (bind _door_activation (Timeline|Door%20Activation Reverse)
          (:Update
            (Transformation|SetRelativeLocation (Variables|Default|GetDoor%20Mesh) (Math|Vector|MakeVector -62.094456 295.442324 _door_activation) false false)))
        (else
          (Timeline|Door%20Activation Play))))))

(event Custom|Switch%20Activated
  (Math|Integer|IncrementInt (Variables|Default|GetPressure%20Switches%20Active)
    (:%20%20
      (if (>= (Variables|Default|GetPressure%20Switches%20Active) 0)
        (bind _door_activation (Timeline|Door%20Activation Play)
          (:Update
            (Transformation|SetRelativeLocation (Variables|Default|GetDoor%20Mesh) (Math|Vector|MakeVector -62.094456 295.442324 _door_activation) false false)))
        (else
          (Timeline|Door%20Activation Reverse))))))

(event Collision|EventActorBeginOverlap
  (params (OtherActor :type Actor%20Object%20Reference)))

(fn ConstructionScript)